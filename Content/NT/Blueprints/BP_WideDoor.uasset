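; BP_WideDoor is a double sliding door that opens for the player character while unlocked.
; Trigger overlap plays or reverses a timeline that slides both panels apart along Y, and both directions are gated by IsUnlocked.
; UnlockDoor and LockDoor set that flag and switch the frame glow and lamps between green and red, stopping or starting warning lamp blinking.
; BeginPlay sets the timeline rate and applies the initial lock visuals.
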(event `self.Trigger.OnComponentBeginOverlap`
  (params (OverlappedComponent :type "PrimitiveComponent Object Reference") (OtherActor :type "Actor Object Reference") (OtherComp :type "PrimitiveComponent Object Reference") (OtherBodyIndex :type Integer) (bFromSweep :type Boolean) (SweepResult :type "HitResult Structure (by ref)"))
  (cast `/Game/NT/Core/Framework/Core_PlayerCharacter` OtherActor)
  (if (`self.IsUnlocked`)
    (bind (_direction _newtrack_0) (`Timeline|Right Door Open` :!label _label)
      (:`Update`
        (`SceneComponent.K2_SetRelativeLocation` (`self.SM_RightDoor`) (`KismetMathLibrary.VLerp` (0.0 0.0 0.0) (0.0 -120.0 0.0) _newtrack_0) false false)
        (`SceneComponent.K2_SetRelativeLocation` (`self.SM_LeftDoor`) (`KismetMathLibrary.VLerp` (0.0 0.0 0.0) (0.0 120.0 0.0) _newtrack_0) false false)))))

(event `self.Trigger.OnComponentEndOverlap`
  (params (OverlappedComponent :type "PrimitiveComponent Object Reference") (OtherActor :type "Actor Object Reference") (OtherComp :type "PrimitiveComponent Object Reference") (OtherBodyIndex :type Integer))
  (cast `/Game/NT/Core/Framework/Core_PlayerCharacter` OtherActor)
  (if (`self.IsUnlocked`)
    (goto _label :!via `Reverse`)))

(event `Unlock Door`
  (set `self.IsUnlocked` true)
  (`PrimitiveComponent.SetMaterial` (`self.SM_DoorFrame`) 6 "/Game/NT/Mateials/M_GreenGlow_Inst.M_GreenGlow_Inst" :!label _label_2)
  (`LightComponent.SetLightColor` (`self.DoorLampRight`) (struct :`G` 0.572917 :`B` 0.043566 :`A` 1.0) true)
  (`LightComponent.SetLightColor` (`self.DoorLampLeft`) (struct :`G` 0.572917 :`B` 0.043566 :`A` 1.0) true)
  (for _array_element (`self.WarningLampArray`)
    (`/Game/NT/Blueprints/BP_WarningLamp.Stop Blink Timer` _array_element)))

(event `self.ReceiveBeginPlay`
  (`TimelineComponent.SetPlayRate` (`self.Right Door Open`) 1.5)
  (if (`self.IsUnlocked`)
    (goto _label_2)
    (else
      (`PrimitiveComponent.SetMaterial` (`self.SM_DoorFrame`) 6 "/Game/NT/Mateials/M_RedGlow_Inst.M_RedGlow_Inst" :!label _label_3)
      (`LightComponent.SetLightColor` (`self.DoorLampRight`) (struct :`R` 1.0 :`A` 1.0) true)
      (`LightComponent.SetLightColor` (`self.DoorLampLeft`) (struct :`R` 1.0 :`A` 1.0) true)
      (for _array_element (`self.WarningLampArray`)
        (`/Game/NT/Blueprints/BP_WarningLamp.Start Blink Timer` _array_element)))))

(event `Lock Door`
  (set `self.IsUnlocked` false)
  (goto _label_3))

(fn `UserConstructionScript`)