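; Physics cube actor that toggles between hanging suspended at a target point and falling under gravity.
; SuspendEvent alternates the states: suspended restores original mass, disables gravity and raises damping; released restores gravity, lowers damping and makes the cube much heavier.
; While suspended, Tick applies a mass-scaled spring force toward TargetPos offset from the actor location.
; BeginPlay caches the starting mass and starts the cube heavy.
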(event `self.ReceiveTick`
  (params (DeltaSeconds :type "Float (single-precision)"))
  (if (`self.SuspensionEnabled`)
    (`PrimitiveComponent.AddForce` (`self.Cube`) (* (- (+ (`self.TargetPos`) (`self.K2_GetActorLocation`)) (`SceneComponent.K2_GetComponentLocation` (`self.Cube`))) (* 70.0 (`PrimitiveComponent.GetMass` (`self.Cube`)))) "None" false)))

(event `SuspendEvent`
  (`/Engine/EditorBlueprintResources/StandardMacros.FlipFlop`
    (:`A`
      (set `self.SuspensionEnabled` true)
      (`PrimitiveComponent.SetEnableGravity` (`self.Cube`) false)
      (`PrimitiveComponent.SetLinearDamping` (`self.Cube`) 3.0)
      (`PrimitiveComponent.SetMassOverrideInKg` (`self.Cube`) "None" (`self.StartMass`) true))
    (:`B`
      (set `self.SuspensionEnabled` false)
      (`PrimitiveComponent.SetEnableGravity` (`self.Cube`) true)
      (`PrimitiveComponent.SetLinearDamping` (`self.Cube`) 0.1)
      (`PrimitiveComponent.SetMassOverrideInKg` (`self.Cube`) "None" (* (`self.StartMass`) 20.0) true))))

(event `self.ReceiveBeginPlay`
  (bind _output_get (set `self.StartMass` (`PrimitiveComponent.GetMass` (`self.Cube`))))
  (`PrimitiveComponent.SetMassOverrideInKg` (`self.Cube`) "None" (* _output_get 20.0) true))

(fn `UserConstructionScript`)