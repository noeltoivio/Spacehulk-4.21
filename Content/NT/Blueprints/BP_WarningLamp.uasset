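; BP_WarningLamp is a warning lamp that blinks red while active and glows green when its blinking is stopped.
; A looping timer created on BeginPlay, paused unless IsBlinking is set, swaps the lamp mesh material to dull red, then to glowing red after a short delay.
; StartBlinkTimer and StopBlinkTimer unpause or pause it, and an active-timer check keeps a pending delay from overriding the green.
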(event `self.ReceiveBeginPlay`
  (bind _returnvalue (`KismetSystemLibrary.K2_SetTimerDelegate` (delegate `Change Material`) 1.0 true))
  (set `self.BlinkTimer` _returnvalue)
  (if (not (`self.IsBlinking`))
    (`KismetSystemLibrary.K2_PauseTimerHandle` (`self.BlinkTimer`))))

(event `Change Material`
  (`PrimitiveComponent.SetMaterial` (`self.SM_Lamp`) 1 "/Game/NT/Mateials/M_Red_Inst.M_Red_Inst")
  (`KismetSystemLibrary.Delay` 0.5)
  (if (`KismetSystemLibrary.K2_IsTimerActiveHandle` (`self.BlinkTimer`))
    (`PrimitiveComponent.SetMaterial` (`self.SM_Lamp`) 1 "/Game/NT/Mateials/M_RedGlow_Inst.M_RedGlow_Inst")))

(event `Start Blink Timer`
  (`KismetSystemLibrary.K2_UnPauseTimerHandle` (`self.BlinkTimer`))
  (set `self.IsBlinking` true))

(event `Stop Blink Timer`
  (`KismetSystemLibrary.K2_PauseTimerHandle` (`self.BlinkTimer`))
  (set `self.IsBlinking` false)
  (`PrimitiveComponent.SetMaterial` (`self.SM_Lamp`) 1 "/Game/NT/Mateials/M_GreenGlow_Inst.M_GreenGlow_Inst"))

(fn `UserConstructionScript`)