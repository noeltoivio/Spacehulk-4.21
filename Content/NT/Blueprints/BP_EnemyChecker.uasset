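; BP_EnemyChecker is a level actor that keeps a large door locked until every larva enemy inside a trigger volume is gone.
; On BeginPlay a looping timer polls the trigger every second for overlapping AI_LarvaPawn actors.
; When none remain, it unlocks the referenced LargeDoor and pauses the timer; until then it prints the remaining count as debug output.
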(event `self.ReceiveBeginPlay`
  (bind _returnvalue (`KismetSystemLibrary.K2_SetTimerDelegate` (delegate `Check For Enemies`) 1.0 true))
  (set `self.Check Timer` _returnvalue)
  (`KismetSystemLibrary.PrintString` "Hello"))

(event `Check For Enemies`
  (bind _returnvalue (`KismetArrayLibrary.Array_Length` (`PrimitiveComponent.GetOverlappingActors` (`self.Trigger`) "/Game/NT/Core/AI/AI_LarvaPawn.AI_LarvaPawn_C")))
  (if (<= _returnvalue 0)
    (`/Game/NT/Blueprints/BP_WideDoor.Unlock Door` (`self.LargeDoor`))
    (`KismetSystemLibrary.K2_PauseTimerHandle` (`self.Check Timer`))
    (`KismetSystemLibrary.PrintString` "All larva is dead! Door is unlocked")
    (else
      (`KismetSystemLibrary.PrintString` (`KismetStringLibrary.Conv_IntToString` _returnvalue)))))

(fn `UserConstructionScript`)