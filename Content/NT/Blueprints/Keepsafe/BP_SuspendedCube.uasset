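; BP_SuspendedCube is a physics cube that can be toggled between floating at a target point and falling freely.
; On BeginPlay it takes player input, and each E press flips suspension, switching gravity and linear damping.
; While suspended, Tick applies a mass-scaled spring force toward TargetPos offset from the actor's location, with the raised damping settling the motion.
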(event `self.ReceiveBeginPlay`
  (`self.EnableInput` (`GameplayStatics.GetPlayerController` 0)))

(event `self.ReceiveTick`
  (params (DeltaSeconds :type "Float (single-precision)"))
  (if (`self.SuspensionEnabled`)
    (`PrimitiveComponent.AddForce` (`self.Cube`) (* (- (+ (`self.TargetPos`) (`self.K2_GetActorLocation`)) (`SceneComponent.K2_GetComponentLocation` (`self.Cube`))) (* 70.0 (`PrimitiveComponent.GetMass` (`self.Cube`)))) "None" false)))

(event `Key|E` :consume false
  (params (Key :type "Key Structure"))
  (:`Pressed`
    (`/Engine/EditorBlueprintResources/StandardMacros.FlipFlop`
      (:`A`
        (set `self.SuspensionEnabled` true)
        (`PrimitiveComponent.SetEnableGravity` (`self.Cube`) false)
        (`PrimitiveComponent.SetLinearDamping` (`self.Cube`) 3.0))
      (:`B`
        (set `self.SuspensionEnabled` false)
        (`PrimitiveComponent.SetEnableGravity` (`self.Cube`) true)
        (`PrimitiveComponent.SetLinearDamping` (`self.Cube`) 0.0)))))

(fn `UserConstructionScript`)