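; BP_Suspended is a physics cube actor that toggles between resting heavy under gravity and floating at a target offset from the actor's location.
; SuspendEvent flip-flops gravity, linear damping and a mass override, restoring normal mass while suspended and a much heavier mass otherwise.
; While suspended, Tick applies a spring-like force toward the target, nudges rotation back toward its starting value and damps angular velocity.
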(event `self.ReceiveBeginPlay`
  ;[1 1 1] Set start values
  (set `self.StartRot` (`SceneComponent.K2_GetComponentRotation` (`self.Cube`)))
  (bind _output_get (set `self.StartMass` (`PrimitiveComponent.GetMass` (`self.Cube`))))
  (`PrimitiveComponent.SetMassOverrideInKg` (`self.Cube`) "None" (* _output_get 20.0) true))

(event `SuspendEvent`
  ;[1 1 1] Toggle between suspension state
  (`/Engine/EditorBlueprintResources/StandardMacros.FlipFlop`
    (:`A`
      (set `self.SuspensionEnabled` true)
      (`PrimitiveComponent.SetEnableGravity` (`self.Cube`) false)
      (`PrimitiveComponent.SetLinearDamping` (`self.Cube`) 3.0)
      (`PrimitiveComponent.SetMassOverrideInKg` (`self.Cube`) "None" (`self.StartMass`) true))
    (:`B`
      (set `self.SuspensionEnabled` false)
      (`PrimitiveComponent.SetEnableGravity` (`self.Cube`) true)
      (`PrimitiveComponent.SetLinearDamping` (`self.Cube`) 0.5)
      (`PrimitiveComponent.SetMassOverrideInKg` (`self.Cube`) "None" (* (`self.StartMass`) 20.0) true))))

(event `self.ReceiveTick`
  (params (DeltaSeconds :type "Float (single-precision)"))
  ;[1 1 1] Make the mesh go to the targeted position
  (if (`self.SuspensionEnabled`)
    (`PrimitiveComponent.AddForce` (`self.Cube`) (* (- (+ (`self.TargetPos`) (`self.K2_GetActorLocation`)) (`SceneComponent.K2_GetComponentLocation` (`self.Cube`))) (* 70.0 (`PrimitiveComponent.GetMass` (`self.Cube`)))) "None" false)
    ;[1 1 1] Set the rotation smoothly
    (`SceneComponent.K2_AddLocalRotation` (`self.Cube`) (* (`KismetMathLibrary.NormalizedDeltaRotator` (`self.StartRot`) (`SceneComponent.K2_GetComponentRotation` (`self.Cube`))) 0.05) false false)
    (`PrimitiveComponent.SetAllPhysicsAngularVelocityInDegrees` (`self.Cube`) (* (`PrimitiveComponent.GetPhysicsAngularVelocityInDegrees` (`self.Cube`) "None") 0.1) false)))

(fn `UserConstructionScript`)